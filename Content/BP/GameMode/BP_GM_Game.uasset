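; Game mode for a two-player card game that manages player joins, deck setup and card draws.
; On login it spawns and possesses a pawn, then a FlipFlop assigns player 1 or 2, spawns both deck views and shuffles that player's list.
; Tick waits for both delayed ready flags, then deals opening hands.
; Draws look up CardDB, move the card from deck to hand, and notify both controllers.
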(event Custom|GM_DrawCard
  (params (PlayerNumber1or2 :type Integer))
  (bind _p2currentdeck (Variables|Default|GetP2CurrentDeck))
  (bind _p1currentdeck (Variables|Default|GetP1CurrentDeck))
  (bind _returnvalue (Utilities|Array|Length _p2currentdeck))
  (bind _returnvalue_2 (Utilities|Array|Length _p1currentdeck))
  (bind _returnvalue_3 (- _returnvalue 1))
  (bind _returnvalue_4 (- _returnvalue_2 1))
  (Variables|Default|SetPlayerToDraw PlayerNumber1or2)
  (if (== (Variables|Default|GetPlayerToDraw) 1)
    ;[1 1 1] Triggers SetupCard on new hand in card, removes from DeckArray and adds to HandArray
    (bind _returnvalue_5 (Utilities|GetDataTableRow "/Game/Data/DataTables/CardDB.CardDB" (Utilities|String|StringToName (Utilities|Array|Get(acopy) (Variables|Default|GetP1CurrentDeck) _returnvalue_4)))
      (:then
        (Default|PCPlayerDrawCard (Utilities|Array|Get(acopy) (Variables|Default|GetPlayer_Controllers)) (Utilities|Text|ToText(String) (.CardName (Utilities|Struct|BreakS_CardInfo _returnvalue_5))) (.Type (Utilities|Struct|BreakS_CardInfo _returnvalue_5)))
        (Utilities|Array|Add (Variables|Default|GetP1CurrentHand) (.CardName (Utilities|Struct|BreakS_CardInfo _returnvalue_5)))
        (Utilities|Array|RemoveIndex (Variables|Default|GetP1CurrentDeck) _returnvalue_4)
        ;[1 1 1] Remove Card from Opponent Deck
        (Default|PCOpponentDrawCard (Utilities|Array|Get(acopy) (Variables|Default|GetPlayer_Controllers) 1))))
    (else
      (bind _returnvalue_6 (Utilities|GetDataTableRow "/Game/Data/DataTables/CardDB.CardDB" (Utilities|String|StringToName (Utilities|Array|Get(acopy) (Variables|Default|GetP2CurrentDeck) _returnvalue_3)))
        (:then
          (Default|PCPlayerDrawCard (Utilities|Array|Get(acopy) (Variables|Default|GetPlayer_Controllers) 1) (Utilities|Text|ToText(String) (.CardName (Utilities|Struct|BreakS_CardInfo _returnvalue_6))) (.Type (Utilities|Struct|BreakS_CardInfo _returnvalue_6)))
          (Utilities|Array|Add (Variables|Default|GetP2CurrentHand) (.CardName (Utilities|Struct|BreakS_CardInfo _returnvalue_6)))
          (Utilities|Array|RemoveIndex (Variables|Default|GetP2CurrentDeck) _returnvalue_3)
          (Default|PCOpponentDrawCard (Utilities|Array|Get(acopy) (Variables|Default|GetPlayer_Controllers))))))))

(event Custom|StartGame
  (CallFunction|DrawOpeningHand))

(event EventTick
  (params (DeltaSeconds :type Float%20%28single-precision%29))
  (if (Variables|Default|GetWaitingToStart)
    (if (Variables|Default|GetP1Ready)
      (if (Variables|Default|GetP2Ready)
        (CallFunction|StartGame)
        (Variables|Default|SetWaitingToStart false)))))

(event EventPostLogin
  (params (NewPlayer :type Player%20Controller%20Object%20Reference))
  (bind _asbp_pc_game (Utilities|Casting|CastToBP_PC_Game NewPlayer))
  (Variables|Default|SetNew%20Player%20Controller _asbp_pc_game)
  (Utilities|Array|Add (Variables|Default|GetPlayer_Controllers) (Variables|Default|GetNew%20Player%20Controller))
  (bind _pawn (CallFunction|SpawnPlayerPawn (Variables|Default|GetNew%20Player%20Controller)))
  (Variables|Default|SetNew%20Player%20Pawn _pawn)
  (Utilities|FlowControl|FlipFlop
    (:A
      ;[1 1 1] Initialize Player 1
      (Default|SpawnPlayerDeck (Variables|Default|GetNew%20Player%20Controller) (Variables|Default|GetNew%20Player%20Pawn) (Utilities|Array|Length (Variables|Default|GetPlayer1CardList)) (Math|Transform|MakeTransform "-135.000000,-325.000000,0.000000" "0.000000,0.000000,180.000000" "1.000000,1.000000,1.000000"))
      (Default|SpawnOpponentDeck (Variables|Default|GetNew%20Player%20Controller) (Variables|Default|GetNew%20Player%20Pawn) (Utilities|Array|Length (Variables|Default|GetPlayer2CardList)) (Math|Transform|MakeTransform "135.000000,325.000000,0.000000" "0.000000,0.000000,180.000000" "1.000000,1.000000,1.000000"))
      (bind _output_get (Variables|Default|SetP1CurrentDeck (Variables|Default|GetPlayer1CardList)))
      (Utilities|Array|Shuffle _output_get)
      (Utilities|FlowControl|Delay 2.0)
      (Variables|Default|SetP1Ready true))
    (:B
      ;[1 1 1] Initialize Player 2
      (Default|SpawnPlayerDeck (Variables|Default|GetNew%20Player%20Controller) (Variables|Default|GetNew%20Player%20Pawn) (Utilities|Array|Length (Variables|Default|GetPlayer2CardList)) (Math|Transform|MakeTransform "-135.000000,-325.000000,0.000000" "0.000000,0.000000,180.000000" "1.000000,1.000000,1.000000"))
      (Default|SpawnOpponentDeck (Variables|Default|GetNew%20Player%20Controller) (Variables|Default|GetNew%20Player%20Pawn) (Utilities|Array|Length (Variables|Default|GetPlayer1CardList)) (Math|Transform|MakeTransform "135.000000,325.000000,0.000000" "0.000000,0.000000,180.000000" "1.000000,1.000000,1.000000"))
      (bind _output_get_2 (Variables|Default|SetP2CurrentDeck (Variables|Default|GetPlayer2CardList)))
      (Utilities|Array|Shuffle _output_get_2)
      (Utilities|FlowControl|Delay 2.0)
      (Variables|Default|SetP2Ready true))))

(event EventOnLogout
  (params (ExitingController :type Controller%20Object%20Reference))
  ;[1 1 1] Probably don't do this. Lol
  (bind _asbp_pc_game (Utilities|Casting|CastToBP_PC_Game ExitingController))
  (Utilities|Array|RemoveItem (Variables|Default|GetPlayer_Controllers) _asbp_pc_game))

(fn ConstructionScript)

(fn SpawnPlayerPawn
  (params (PlayerController :type Player%20Controller%20Object%20Reference))
  (Utilities|IsValid (Pawn|GetControlledPawn PlayerController)
    (:Is%20Valid
      (Actor|DestroyActor PlayerController))
    (:Is%20Not%20Valid
      _))
  (bind _returnvalue (Game|SpawnActorfromClass "/Game/BP/Pawns/BP_Pawn_Game.BP_Pawn_Game_C" (Math|Transform|MakeTransform "0, 0, 0" "0, 0, 0" "1.000000,1.000000,1.000000") "AlwaysSpawn" "MultiplyWithRoot" PlayerController 0))
  (Pawn|Possess PlayerController _returnvalue)
  (return _returnvalue))

(fn DrawOpeningHand
  (for _index (range 0 6)
    (CallFunction|GMDrawCard 1)
    (CallFunction|GMDrawCard 2)))