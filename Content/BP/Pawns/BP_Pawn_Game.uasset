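; Game pawn for a card game, with a spring-arm camera and a CastBox zone that signals casting intent.
; A BP_A_Card entering CastBox sets WantsToCast on BP_PC_Game, and any end overlap clears it without checking the actor type.
; Disconnected dev-only nodes remain for nudging camera FOV and spring-arm position and pitch, and for printing the arm's transform.
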(event OnComponentBeginOverlap(CastBox)
  (params (OverlappedComponent :type Primitive%20Component%20Object%20Reference) (OtherActor :type Actor%20Object%20Reference) (OtherComp :type Primitive%20Component%20Object%20Reference) (OtherBodyIndex :type Integer) (bFromSweep :type Boolean) (SweepResult :type Hit%20Result%20Structure%20%28by%20ref%29))
  (Utilities|Casting|CastToBP_A_Card OtherActor)
  (bind _asbp_pc_game (Utilities|Casting|CastToBP_PC_Game (Game|GetPlayerController 0)))
  (Variables|/Game/BP/PlayerController/BP_PC_Game.BP_PC_Game_C|SetWantsToCast _asbp_pc_game true))

(event OnComponentEndOverlap(CastBox)
  (params (OverlappedComponent :type Primitive%20Component%20Object%20Reference) (OtherActor :type Actor%20Object%20Reference) (OtherComp :type Primitive%20Component%20Object%20Reference) (OtherBodyIndex :type Integer))
  (bind _asbp_pc_game (Utilities|Casting|CastToBP_PC_Game (Game|GetPlayerController 0)))
  (Variables|/Game/BP/PlayerController/BP_PC_Game.BP_PC_Game_C|SetWantsToCast _asbp_pc_game false))

(event Input|KeyboardEvents|Q
  (params (Key :type Key%20Structure :default "None"))
  ;[1 1 1] These help position the camera. Dev only
)

(event Input|KeyboardEvents|W
  (params (Key :type Key%20Structure :default "None"))
  ;[1 1 1] These help position the camera. Dev only
)

(event Input|KeyboardEvents|P
  (params (Key :type Key%20Structure :default "None"))
  ;[1 1 1] These help position the camera. Dev only
)

(event Input|KeyboardEvents|A
  (params (Key :type Key%20Structure :default "None"))
  ;[1 1 1] These help position the camera. Dev only
)

(event Input|KeyboardEvents|S
  (params (Key :type Key%20Structure :default "None"))
  ;[1 1 1] These help position the camera. Dev only
)

(event Input|KeyboardEvents|Z
  (params (Key :type Key%20Structure :default "None"))
  ;[1 1 1] These help position the camera. Dev only
)

(event Input|KeyboardEvents|X
  (params (Key :type Key%20Structure :default "None"))
  ;[1 1 1] These help position the camera. Dev only
)

(event Input|KeyboardEvents|E
  (params (Key :type Key%20Structure :default "None"))
  ;[1 1 1] These help position the camera. Dev only
)

(event Input|KeyboardEvents|D
  (params (Key :type Key%20Structure :default "None"))
  ;[1 1 1] These help position the camera. Dev only
)

(fn ConstructionScript)