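; BP_A_Card is a card actor with a Cube component and text renders for its labels.
; SetupCard writes the card name to the middle text and the card type to the bottom text.
; Other events store the card state and change the Cube's collision response on a given channel.
; Getter functions report a fixed actor type and the card's index in the hand array.
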(event Custom|SetupCard
  (params (Card%20Name :type Text%20%28by%20ref%29) (Card%20Type :type E_CardTypes%20Enum :default "NewEnumerator0"))
  (Rendering|Components|TextRender|SetText (Variables|Default|GetMiddleTextRender) Card%20Name)
  (Rendering|Components|TextRender|SetText (Variables|Default|GetBottomRender) (Utilities|Text|ToText(String) (Utilities|String|EnumtoString Card%20Type))))

(event EventChangeCollisionResponse
  (params (Channel :type ECollisionChannel%20Enum :default "ECC_WorldStatic") (Resposne :type ECollisionResponse%20Enum :default "ECR_Ignore"))
  (Collision|SetCollisionResponsetoChannel (Variables|Default|GetCube) Channel Resposne))

(event EventSetCardState
  (params (CardState :type E_CardStates%20Enum :default "NewEnumerator0"))
  (Variables|Default|SetCardState CardState))

(fn ConstructionScript)

(fn GetActorType
  (return "NewEnumerator0"))

(fn GetHandArrayIndexOfCard
  (return (Variables|Default|GetHandArrayIndex)))