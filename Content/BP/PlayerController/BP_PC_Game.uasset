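; Player controller for a card game that spawns both decks as stacked card actors, moves draws into hand arrays and handles mouse interaction.
; A Searching/Viewing/Holding state machine uses cursor traces to preview and drag cards, swapping hand order when dragged over another.
; Each Tick interpolates cards toward fanned hand, view or drag transforms, toggling trace-channel responses during moves.
; Opponent cards have collision disabled after spawning; CastCard only prints a placeholder.
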(event Custom|SpawnOpponentDeck
  (params (Pawn :type Pawn%20Object%20Reference) (NumberOfCardsInDeck :type Integer) (LocalDeckLocation :type Transform))
  ;[1 1 1] Spawns Card Actors In A Stack @ Location
  (bind _asbp_pawn_game (Utilities|Casting|CastToBP_Pawn_Game Pawn))
  (for _index (range 0 (- NumberOfCardsInDeck 1))
    (bind _returnvalue (Game|SpawnActorfromClass "/Game/BP/Actors/BP_A_Card.BP_A_Card_C" (Math|Transform|MakeTransform (Math|Vector|MakeVector (.x (.location LocalDeckLocation)) (.y (.location LocalDeckLocation)) (+ (.z (.location LocalDeckLocation)) (* _index 0.45) 0.25)) (.rotation LocalDeckLocation) (.scale LocalDeckLocation)) "AlwaysSpawn" "MultiplyWithRoot" _asbp_pawn_game 0))
    (Utilities|Array|Add (Variables|Default|GetOpponentDeckArray) _returnvalue))
  (CallFunction|ClearCollision))

(event Custom|SpawnPlayerDeck
  (params (Pawn :type Pawn%20Object%20Reference) (NumberOfCardsInDeck :type Integer) (LocalDeckLocation :type Transform))
  ;[1 1 1] Spawns Card Actors In A Stack @ Location
  (bind _asbp_pawn_game (Utilities|Casting|CastToBP_Pawn_Game Pawn))
  (for _index (range 0 (- NumberOfCardsInDeck 1))
    (bind _returnvalue (Game|SpawnActorfromClass "/Game/BP/Actors/BP_A_Card.BP_A_Card_C" (Math|Transform|MakeTransform (Math|Vector|MakeVector (.x (.location LocalDeckLocation)) (.y (.location LocalDeckLocation)) (+ (.z (.location LocalDeckLocation)) (* _index 0.45) 0.25)) (.rotation LocalDeckLocation) (.scale LocalDeckLocation)) "AlwaysSpawn" "MultiplyWithRoot" _asbp_pawn_game 0))
    (Utilities|Array|Add (Variables|Default|GetPlayerDeckArray) _returnvalue)))

(event Custom|Clear%20Collision
  ;[1 1 1] Stops player mouse from triggering on opponent cards
  (Utilities|FlowControl|Delay 0.5)
  (for _array_element (Variables|Default|GetOpponentDeckArray)
    (Collision|SetCollisionEnabled (Variables|/Game/BP/Actors/BP_A_Card.BP_A_Card_C|GetCube _array_element) "NoCollision")))

(event Custom|PC_PlayerDrawCard
  (params (Card%20Name :type Text%20%28by%20ref%29) (Card%20Type :type E_CardTypes%20Enum :default "NewEnumerator0"))
  (bind _playerdeckarray (Variables|Default|GetPlayerDeckArray))
  (bind _playerdeckarray_2 (Variables|Default|GetPlayerDeckArray))
  (bind _returnvalue (Utilities|Array|Length _playerdeckarray_2))
  (bind _returnvalue_2 (- _returnvalue 1))
  (bind _output (Utilities|Array|Get(acopy) _playerdeckarray _returnvalue_2))
  ;[1 1 1] Adjusts the card actors representations on each player
  (Default|SetupCard _output Card%20Name Card%20Type)
  (Utilities|Array|Add (Variables|Default|GetPlayerHandArray) _output)
  (Utilities|Array|RemoveIndex (Variables|Default|GetPlayerDeckArray) _returnvalue_2))

(event Custom|PC_OpponentDrawCard
  (bind _opponentdeckarray (Variables|Default|GetOpponentDeckArray))
  (bind _returnvalue (Utilities|Array|Length _opponentdeckarray))
  (bind _returnvalue_2 (- _returnvalue 1))
  ;[1 1 1] Adjusts the card actors representations on each player
  (Utilities|Array|Add (Variables|Default|GetOpponentHandArray) (Utilities|Array|Get(acopy) _opponentdeckarray _returnvalue_2))
  (Utilities|Array|RemoveIndex _opponentdeckarray _returnvalue_2))

(event EventTick
  (params (DeltaSeconds :type Float%20%28single-precision%29))
  (CardUI|RunPlayerCardUI)
  (CardUI|RunOpponentCardUI)
  (switch Utilities|FlowControl|Switch|SwitchonE_HandleStates (Variables|Default|GetHandleState)
    (:NewEnumerator0
      (StateFunctions|SearchingStateFunction))
    (:NewEnumerator1
      (StateFunctions|ViewingStateFunction))
    (:NewEnumerator2
      (StateFunctions|HoldingStateFunction))))

(event EventBeginPlay
  (Variables|Default|SetbShowMouseCursor true))

(event Input|MouseEvents|LeftMouseButton
  (params (Key :type Key%20Structure :default "None"))
  (:Pressed
    (if (Utilities|Enum|Equal(Enum) (Variables|Default|GetHandleState) "NewEnumerator1")
      (Variables|Default|SetHandleState "NewEnumerator2")
      (Class|BPInterfaceFunctions|SetCardState(Message) (Variables|Default|GetCurrentViewedCard) "NewEnumerator2")))
  (:Released
    (if (Utilities|Enum|Equal(Enum) (Variables|Default|GetHandleState) "NewEnumerator2")
      (if (Variables|Default|GetWantsToCast)
        (CallFunction|CastCard)
        (Variables|Default|SetHandleState "NewEnumerator0")
        (Class|BPInterfaceFunctions|SetCardState(Message) (Variables|Default|GetCurrentViewedCard) "NewEnumerator0")
        (else
          (Variables|Default|SetHandleState "NewEnumerator0")
          (Class|BPInterfaceFunctions|SetCardState(Message) (Variables|Default|GetCurrentViewedCard) "NewEnumerator0")))
      (Class|BPInterfaceFunctions|ChangeCollisionResponse(Message) (Variables|Default|GetCurrentViewedCard) "ECC_GameTraceChannel1" "ECR_Block")
      (Class|BPInterfaceFunctions|ChangeCollisionResponse(Message) (Variables|Default|GetCurrentViewedCard) "ECC_GameTraceChannel2" "ECR_Block"))))

(fn ConstructionScript)

(fn RunPlayerCardUI
  (bind _asbp_pawn_game (Utilities|Casting|CastToBP_Pawn_Game (Game|Player|GetPlayerPawn 0)))
  (LocalVariables|SetPlayerPawn _asbp_pawn_game)
  (for (_array_element _array_index) (Variables|Default|GetPlayerHandArray)
    (Variables|/Game/BP/Actors/BP_A_Card.BP_A_Card_C|SetHandArrayIndex _array_element _array_index)
    (Variables|Default|SetCardIndexInHand _array_index)
    (bind _output_get (Variables|Default|SetCard _array_element))
    (switch Utilities|FlowControl|Switch|SwitchonE_CardStates (Variables|/Game/BP/Actors/BP_A_Card.BP_A_Card_C|GetCardState _output_get)
      (:NewEnumerator0
        ;[1 1 1] Display Cards in Hand
        (Variables|Default|SetHandSize (Utilities|Array|Length (Variables|Default|GetPlayerHandArray)))
        (InterpFunctions|InterpCardTransform (Variables|Default|GetCard) (Variables|Default|GetMoveSpeed) (Math|Vector|MakeVector (- (.x (Transformation|GetWorldLocation (Variables|/Game/BP/Pawns/BP_Pawn_Game.BP_Pawn_Game_C|GetPlayer1HandLocation (LocalVariables|GetPlayerPawn)))) (* (Math|Float|Absolute(Float) (+ (.y (Transformation|GetWorldLocation (Variables|/Game/BP/Pawns/BP_Pawn_Game.BP_Pawn_Game_C|GetPlayer1HandLocation (LocalVariables|GetPlayerPawn)))) (- (Variables|Default|GetCardIndexInHand) (+ (/ (Variables|Default|GetHandSize) 2) (* (- (Math|Integer|%(Integer) (Variables|Default|GetHandSize) 2) 1) 0.5))))) (Variables|Default|GetHandXOffset) (* (Math|Float|Absolute(Float) (+ (.y (Transformation|GetWorldLocation (Variables|/Game/BP/Pawns/BP_Pawn_Game.BP_Pawn_Game_C|GetPlayer1HandLocation (LocalVariables|GetPlayerPawn)))) (- (Variables|Default|GetCardIndexInHand) (+ (/ (Variables|Default|GetHandSize) 2) (* (- (Math|Integer|%(Integer) (Variables|Default|GetHandSize) 2) 1) 0.5))))) 0.1))) (* (+ (.y (Transformation|GetWorldLocation (Variables|/Game/BP/Pawns/BP_Pawn_Game.BP_Pawn_Game_C|GetPlayer1HandLocation (LocalVariables|GetPlayerPawn)))) (- (Variables|Default|GetCardIndexInHand) (+ (/ (Variables|Default|GetHandSize) 2) (* (- (Math|Integer|%(Integer) (Variables|Default|GetHandSize) 2) 1) 0.5)))) (Variables|Default|GetHandYOffset)) (.z (Transformation|GetWorldLocation (Variables|/Game/BP/Pawns/BP_Pawn_Game.BP_Pawn_Game_C|GetPlayer1HandLocation (LocalVariables|GetPlayerPawn))))) (Math|Rotator|MakeRotator 0.0 2e+01 (* (+ (.y (Transformation|GetWorldLocation (Variables|/Game/BP/Pawns/BP_Pawn_Game.BP_Pawn_Game_C|GetPlayer1HandLocation (LocalVariables|GetPlayerPawn)))) (- (Variables|Default|GetCardIndexInHand) (+ (/ (Variables|Default|GetHandSize) 2) (* (- (Math|Integer|%(Integer) (Variables|Default|GetHandSize) 2) 1) 0.5)))) 0.4)) "1.000000,1.000000,1.000000"))
      (:NewEnumerator1
        ;[1 1 1] View Card
        (Variables|Default|SetHandSize (Utilities|Array|Length (Variables|Default|GetPlayerHandArray)))
        (InterpFunctions|InterpCardTransform (Variables|Default|GetCard) (Variables|Default|GetMoveSpeed) (/ (Math|Vector|MakeVector (+ (.x (+ (Transformation|GetWorldLocation (Variables|/Game/BP/Pawns/BP_Pawn_Game.BP_Pawn_Game_C|GetCamera (LocalVariables|GetPlayerPawn))) (Math|Vector|MakeVector (- (.x (Transformation|GetWorldLocation (Variables|/Game/BP/Pawns/BP_Pawn_Game.BP_Pawn_Game_C|GetPlayer1HandLocation (LocalVariables|GetPlayerPawn)))) (* (Math|Float|Absolute(Float) (+ (.y (Transformation|GetWorldLocation (Variables|/Game/BP/Pawns/BP_Pawn_Game.BP_Pawn_Game_C|GetPlayer1HandLocation (LocalVariables|GetPlayerPawn)))) (- (Variables|Default|GetCardIndexInHand) (+ (/ (Variables|Default|GetHandSize) 2) (* (- (Math|Integer|%(Integer) (Variables|Default|GetHandSize) 2) 1) 0.5))))) (Variables|Default|GetHandXOffset))) (* (+ (.y (Transformation|GetWorldLocation (Variables|/Game/BP/Pawns/BP_Pawn_Game.BP_Pawn_Game_C|GetPlayer1HandLocation (LocalVariables|GetPlayerPawn)))) (- (Variables|Default|GetCardIndexInHand) (+ (/ (Variables|Default|GetHandSize) 2) (* (- (Math|Integer|%(Integer) (Variables|Default|GetHandSize) 2) 1) 0.5)))) (Variables|Default|GetHandYOffset)) (.z (Transformation|GetWorldLocation (Variables|/Game/BP/Pawns/BP_Pawn_Game.BP_Pawn_Game_C|GetPlayer1HandLocation (LocalVariables|GetPlayerPawn))))))) (+ (* (Math|Float|Absolute(Float) (+ (.y (Transformation|GetWorldLocation (Variables|/Game/BP/Pawns/BP_Pawn_Game.BP_Pawn_Game_C|GetPlayer1HandLocation (LocalVariables|GetPlayerPawn)))) (- (Variables|Default|GetCardIndexInHand) (+ (/ (Variables|Default|GetHandSize) 2) (* (- (Math|Integer|%(Integer) (Variables|Default|GetHandSize) 2) 1) 0.5))))) (Variables|Default|GetHandXOffset)) 38.0)) (.y (+ (Transformation|GetWorldLocation (Variables|/Game/BP/Pawns/BP_Pawn_Game.BP_Pawn_Game_C|GetCamera (LocalVariables|GetPlayerPawn))) (Math|Vector|MakeVector (- (.x (Transformation|GetWorldLocation (Variables|/Game/BP/Pawns/BP_Pawn_Game.BP_Pawn_Game_C|GetPlayer1HandLocation (LocalVariables|GetPlayerPawn)))) (* (Math|Float|Absolute(Float) (+ (.y (Transformation|GetWorldLocation (Variables|/Game/BP/Pawns/BP_Pawn_Game.BP_Pawn_Game_C|GetPlayer1HandLocation (LocalVariables|GetPlayerPawn)))) (- (Variables|Default|GetCardIndexInHand) (+ (/ (Variables|Default|GetHandSize) 2) (* (- (Math|Integer|%(Integer) (Variables|Default|GetHandSize) 2) 1) 0.5))))) (Variables|Default|GetHandXOffset))) (* (+ (.y (Transformation|GetWorldLocation (Variables|/Game/BP/Pawns/BP_Pawn_Game.BP_Pawn_Game_C|GetPlayer1HandLocation (LocalVariables|GetPlayerPawn)))) (- (Variables|Default|GetCardIndexInHand) (+ (/ (Variables|Default|GetHandSize) 2) (* (- (Math|Integer|%(Integer) (Variables|Default|GetHandSize) 2) 1) 0.5)))) (Variables|Default|GetHandYOffset)) (.z (Transformation|GetWorldLocation (Variables|/Game/BP/Pawns/BP_Pawn_Game.BP_Pawn_Game_C|GetPlayer1HandLocation (LocalVariables|GetPlayerPawn))))))) (.z (+ (Transformation|GetWorldLocation (Variables|/Game/BP/Pawns/BP_Pawn_Game.BP_Pawn_Game_C|GetCamera (LocalVariables|GetPlayerPawn))) (Math|Vector|MakeVector (- (.x (Transformation|GetWorldLocation (Variables|/Game/BP/Pawns/BP_Pawn_Game.BP_Pawn_Game_C|GetPlayer1HandLocation (LocalVariables|GetPlayerPawn)))) (* (Math|Float|Absolute(Float) (+ (.y (Transformation|GetWorldLocation (Variables|/Game/BP/Pawns/BP_Pawn_Game.BP_Pawn_Game_C|GetPlayer1HandLocation (LocalVariables|GetPlayerPawn)))) (- (Variables|Default|GetCardIndexInHand) (+ (/ (Variables|Default|GetHandSize) 2) (* (- (Math|Integer|%(Integer) (Variables|Default|GetHandSize) 2) 1) 0.5))))) (Variables|Default|GetHandXOffset))) (* (+ (.y (Transformation|GetWorldLocation (Variables|/Game/BP/Pawns/BP_Pawn_Game.BP_Pawn_Game_C|GetPlayer1HandLocation (LocalVariables|GetPlayerPawn)))) (- (Variables|Default|GetCardIndexInHand) (+ (/ (Variables|Default|GetHandSize) 2) (* (- (Math|Integer|%(Integer) (Variables|Default|GetHandSize) 2) 1) 0.5)))) (Variables|Default|GetHandYOffset)) (.z (Transformation|GetWorldLocation (Variables|/Game/BP/Pawns/BP_Pawn_Game.BP_Pawn_Game_C|GetPlayer1HandLocation (LocalVariables|GetPlayerPawn)))))))) 2.0) (Math|Rotator|MakeRotator 0.0 15.0 0.0) "1.000000,1.000000,1.000000"))
      (:NewEnumerator2
        ;[1 1 1] Drag Card
        (Class|BPInterfaceFunctions|ChangeCollisionResponse(Message) (Variables|Default|GetCard) "ECC_GameTraceChannel2" "ECR_Ignore")
        (Class|BPInterfaceFunctions|ChangeCollisionResponse(Message) (Variables|Default|GetCard) "ECC_GameTraceChannel1" "ECR_Block")
        (bind _out_location (CardUI|GetUnderMouse "TraceTypeQuery4"))
        (InterpFunctions|InterpCardTransform (Variables|Default|GetCard) (Variables|Default|GetMoveSpeed) (/ (+ (Transformation|GetWorldLocation (Variables|/Game/BP/Pawns/BP_Pawn_Game.BP_Pawn_Game_C|GetCamera (LocalVariables|GetPlayerPawn))) _out_location) 2.0) "0, 0, 0" "1.000000,1.000000,1.000000")))))

(fn SearchingStateFunction
  (bind _out_actor (CardUI|GetUnderMouse "TraceTypeQuery3"))
  (bind _actortype (Class|BPInterfaceFunctions|GetActorType(Message) _out_actor))
  (if (Utilities|Enum|Equal(Enum) _actortype "NewEnumerator0")
    (Variables|Default|SetHandleState "NewEnumerator1")
    (Class|BPInterfaceFunctions|SetCardState(Message) _out_actor "NewEnumerator1")
    (Variables|Default|SetCurrentViewedCard _out_actor)))

(fn ViewingStateFunction
  (bind _currentviewedcard (Variables|Default|GetCurrentViewedCard))
  (bind _out_actor (CardUI|GetUnderMouse "TraceTypeQuery3"))
  (if (not (== _out_actor _currentviewedcard))
    (Variables|Default|SetHandleState "NewEnumerator0")
    (Class|BPInterfaceFunctions|SetCardState(Message) _currentviewedcard "NewEnumerator0")))

(fn HoldingStateFunction
  (bind _out_actor (CardUI|GetUnderMouse "TraceTypeQuery4"))
  (Variables|Default|SetHitCard _out_actor)
  (bind _actortype (Class|BPInterfaceFunctions|GetActorType(Message) (Variables|Default|GetHitCard)))
  (if (Utilities|Enum|Equal(Enum) _actortype "NewEnumerator0")
    (bind _index (Class|BPInterfaceFunctions|GetHandArrayIndexOfCard(Message) (Variables|Default|GetHitCard)))
    (bind _index_2 (Class|BPInterfaceFunctions|GetHandArrayIndexOfCard(Message) (Variables|Default|GetCurrentViewedCard)))
    (Variables|Default|SetCurrentViewedCardIndex _index_2)
    (if (!= (- (Variables|Default|GetCurrentViewedCardIndex) _index) 0)
      (Variables|Default|SetOffsetToMoveCard (- (Variables|Default|GetCurrentViewedCardIndex) _index))
      (Class|BPInterfaceFunctions|ChangeCollisionResponse(Message) (Variables|Default|GetHitCard) "ECC_GameTraceChannel2" "ECR_Ignore")
      (Variables|Default|SetNumberOfCardsToMove (Math|Integer|Absolute(Integer) (Variables|Default|GetOffsetToMoveCard)))
      (while (!= (Variables|Default|GetNumberOfCardsToMove) 0)
        (if (> (Variables|Default|GetOffsetToMoveCard) 0)
          (Utilities|Array|Swap (Variables|Default|GetPlayerHandArray) (Variables|Default|GetCurrentViewedCardIndex) (- (Variables|Default|GetCurrentViewedCardIndex) (Variables|Default|GetNumberOfCardsToMove)))
          (Math|Integer|DecrementInt (Variables|Default|GetNumberOfCardsToMove))
          (else
            (Utilities|Array|Swap (Variables|Default|GetPlayerHandArray) (Variables|Default|GetCurrentViewedCardIndex) (+ (Variables|Default|GetCurrentViewedCardIndex) (Variables|Default|GetNumberOfCardsToMove)))
            (Math|Integer|DecrementInt (Variables|Default|GetNumberOfCardsToMove))))))))

(fn InterpCardTransform
  (params (Card :type BP%20A%20Card%20Object%20Reference) (MoveSpeed :type Float%20%28double-precision%29) (Location :type Vector) (Rotation :type Rotator) (Scale :type Vector))
  (bind (_outlocation _movecomplete) (InterpFunctions|InterpLocation Card MoveSpeed Location))
  (bind (_outrotation _movecomplete_2) (InterpFunctions|InterpRotation Card MoveSpeed Rotation))
  (bind (_outscale _movecomplete_3) (InterpFunctions|InterpScale Card MoveSpeed Scale))
  (Transformation|SetActorTransform Card (Math|Transform|MakeTransform _outlocation _outrotation _outscale))
  (if (Math|Boolean|ANDBoolean _movecomplete _movecomplete_2 _movecomplete_3)
    (Class|BPInterfaceFunctions|ChangeCollisionResponse(Message) Card "ECC_GameTraceChannel2" "ECR_Block")))

(fn GetUnderMouse
  (params (TraceChannel :type ETraceTypeQuery%20Enum :default "TraceTypeQuery1"))
  (bind _returnvalue (Game|GetPlayerController 0))
  (bind (_worldlocation _worlddirection) (Game|Player|ConvertMouseLocationToWorldSpace _returnvalue))
  (bind _outhit (Collision|LineTraceByChannel _worldlocation (+ _worldlocation (* _worlddirection 1e+04)) TraceChannel false 0 "None" false "(R=0.000000,G=0.418566,B=1.000000,A=1.000000)"))
  (return (.location _outhit) (.hitactor _outhit)))

(fn InterpLocation
  (params (Card :type Actor%20Object%20Reference) (MoveSpeed :type Float%20%28double-precision%29) (Target%20Location :type Vector))
  (bind _returnvalue (Transformation|GetActorLocation Card))
  (if (Utilities|Operators|EqualEqual (Math|Vector|MakeVector (.x _returnvalue) (.y _returnvalue) (.z _returnvalue)) (Math|Vector|MakeVector (.x Target%20Location) (.y Target%20Location) (.z Target%20Location)) 0.001)
    (LocalVariables|SetInterpLocationOut (Math|Vector|MakeVector (.x Target%20Location) (.y Target%20Location) (.z Target%20Location)))
    (LocalVariables|SetIsMoveComplete true)
    (else
      (LocalVariables|SetInterpLocationOut (Math|Vector|MakeVector (Math|Interpolation|FInterpTo (.x _returnvalue) (.x Target%20Location) (Utilities|Time|GetWorldDeltaSeconds) MoveSpeed) (Math|Interpolation|FInterpTo (.y _returnvalue) (.y Target%20Location) (Utilities|Time|GetWorldDeltaSeconds) MoveSpeed) (Math|Interpolation|FInterpTo (.z _returnvalue) (.z Target%20Location) (Utilities|Time|GetWorldDeltaSeconds) MoveSpeed)))
      (LocalVariables|SetIsMoveComplete false)))
  (return (LocalVariables|GetInterpLocationOut) (LocalVariables|GetIsMoveComplete)))

(fn InterpRotation
  (params (Card :type Actor%20Object%20Reference) (MoveSpeed :type Float%20%28double-precision%29) (Target%20Rotation :type Rotator))
  (bind _returnvalue (Math|Rotator|MakeRotator (.roll Target%20Rotation) (.pitch Target%20Rotation) (.yaw Target%20Rotation)))
  (bind _returnvalue_2 (Transformation|GetActorRotation Card))
  (if (Utilities|Operators|EqualEqual (Math|Rotator|MakeRotator (.roll _returnvalue_2) (.pitch _returnvalue_2) (.yaw _returnvalue_2)) _returnvalue 0.001)
    (LocalVariables|SetInterpRotationOut _returnvalue)
    (LocalVariables|SetIsMoveComplete true)
    (else
      (LocalVariables|SetInterpRotationOut (Math|Rotator|MakeRotator (Math|Interpolation|FInterpTo (.roll _returnvalue_2) (.roll Target%20Rotation) (Utilities|Time|GetWorldDeltaSeconds) MoveSpeed) (Math|Interpolation|FInterpTo (.pitch _returnvalue_2) (.pitch Target%20Rotation) (Utilities|Time|GetWorldDeltaSeconds) MoveSpeed) (Math|Interpolation|FInterpTo (.yaw _returnvalue_2) (.yaw Target%20Rotation) (Utilities|Time|GetWorldDeltaSeconds) MoveSpeed)))
      (LocalVariables|SetIsMoveComplete false)))
  (return (LocalVariables|GetInterpRotationOut) (LocalVariables|GetIsMoveComplete)))

(fn InterpScale
  (params (Card :type Actor%20Object%20Reference) (MoveSpeed :type Float%20%28double-precision%29) (Target%20Scale :type Vector))
  (bind _returnvalue (Math|Vector|MakeVector (.x Target%20Scale) (.y Target%20Scale) (.z Target%20Scale)))
  (bind _returnvalue_2 (Transformation|GetActorScale3D Card))
  (if (Utilities|Operators|EqualEqual (Math|Vector|MakeVector (.x _returnvalue_2) (.y _returnvalue_2) (.z _returnvalue_2)) _returnvalue 0.001)
    (LocalVariables|SetInterpScaleOut _returnvalue)
    (LocalVariables|SetIsMoveComplete true)
    (else
      (LocalVariables|SetInterpScaleOut (Math|Vector|MakeVector (Math|Interpolation|FInterpTo (.x _returnvalue_2) (.x Target%20Scale) (Utilities|Time|GetWorldDeltaSeconds) MoveSpeed) (Math|Interpolation|FInterpTo (.y _returnvalue_2) (.y Target%20Scale) (Utilities|Time|GetWorldDeltaSeconds) MoveSpeed) (Math|Interpolation|FInterpTo (.z _returnvalue_2) (.z Target%20Scale) (Utilities|Time|GetWorldDeltaSeconds) MoveSpeed)))
      (LocalVariables|SetIsMoveComplete false)))
  (return (LocalVariables|GetInterpScaleOut) (LocalVariables|GetIsMoveComplete)))

(fn CastCard
  (Development|PrintString "CAST"))

(fn RunOpponentCardUI
  (bind _asbp_pawn_game (Utilities|Casting|CastToBP_Pawn_Game (Game|Player|GetPlayerPawn 0)))
  (LocalVariables|SetPlayerPawn _asbp_pawn_game)
  (for (_array_element _array_index) (Variables|Default|GetOpponentHandArray)
    (Variables|/Game/BP/Actors/BP_A_Card.BP_A_Card_C|SetHandArrayIndex _array_element _array_index)
    (Variables|Default|SetCardIndexInHand _array_index)
    (Variables|Default|SetCard _array_element)
    ;[1 1 1] Display Cards in Hand
    (Variables|Default|SetHandSize (Utilities|Array|Length (Variables|Default|GetOpponentHandArray)))
    (InterpFunctions|InterpCardTransform (Variables|Default|GetCard) (Variables|Default|GetMoveSpeed) (Math|Vector|MakeVector (- (.x (Transformation|GetWorldLocation (Variables|/Game/BP/Pawns/BP_Pawn_Game.BP_Pawn_Game_C|GetPlayer2HandLocation (LocalVariables|GetPlayerPawn)))) (* (* (Math|Float|Absolute(Float) (+ (.y (Transformation|GetWorldLocation (Variables|/Game/BP/Pawns/BP_Pawn_Game.BP_Pawn_Game_C|GetPlayer2HandLocation (LocalVariables|GetPlayerPawn)))) (- (Variables|Default|GetCardIndexInHand) (+ (/ (Variables|Default|GetHandSize) 2) (* (- (Math|Integer|%(Integer) (Variables|Default|GetHandSize) 2) 1) 0.5))))) (Variables|Default|GetHandXOffset) (* (Math|Float|Absolute(Float) (+ (.y (Transformation|GetWorldLocation (Variables|/Game/BP/Pawns/BP_Pawn_Game.BP_Pawn_Game_C|GetPlayer2HandLocation (LocalVariables|GetPlayerPawn)))) (- (Variables|Default|GetCardIndexInHand) (+ (/ (Variables|Default|GetHandSize) 2) (* (- (Math|Integer|%(Integer) (Variables|Default|GetHandSize) 2) 1) 0.5))))) 0.1)) -1.0)) (* (+ (.y (Transformation|GetWorldLocation (Variables|/Game/BP/Pawns/BP_Pawn_Game.BP_Pawn_Game_C|GetPlayer2HandLocation (LocalVariables|GetPlayerPawn)))) (- (Variables|Default|GetCardIndexInHand) (+ (/ (Variables|Default|GetHandSize) 2) (* (- (Math|Integer|%(Integer) (Variables|Default|GetHandSize) 2) 1) 0.5)))) (Variables|Default|GetHandYOffset)) (.z (Transformation|GetWorldLocation (Variables|/Game/BP/Pawns/BP_Pawn_Game.BP_Pawn_Game_C|GetPlayer2HandLocation (LocalVariables|GetPlayerPawn))))) (Math|Rotator|MakeRotator 0.0 -2e+01 (* (+ (.y (Transformation|GetWorldLocation (Variables|/Game/BP/Pawns/BP_Pawn_Game.BP_Pawn_Game_C|GetPlayer2HandLocation (LocalVariables|GetPlayerPawn)))) (- (Variables|Default|GetCardIndexInHand) (+ (/ (Variables|Default|GetHandSize) 2) (* (- (Math|Integer|%(Integer) (Variables|Default|GetHandSize) 2) 1) 0.5)))) -0.4)) "1.000000,1.000000,1.000000")))